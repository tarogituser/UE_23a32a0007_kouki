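; BP_ObjectBase is a base trigger object that starts a linked moving object when an actor overlaps its Box.
; The overlap calls an event dispatcher, bound to its own handler on BeginPlay, which casts TargetObject to BP_MovingObject and starts it.
; Only if that cast succeeds, the overlapping actor receives MyCharacterOverlapMessage with this object's name and zero points.
; A separate DestroyObject event removes the actor.
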(event OnComponentBeginOverlap(Box)
  (params (OverlappedComponent :type Primitive%20Component%20Object%20Reference) (OtherActor :type Actor%20Object%20Reference) (OtherComp :type Primitive%20Component%20Object%20Reference) (OtherBodyIndex :type Integer) (bFromSweep :type Boolean) (SweepResult :type Hit%20Result%20Structure%20%28by%20ref%29))
  (Default|CallOverlapBaseEventAction OtherActor))

(event Custom|OverlapBaseEvent
  (params (OverlapActor :type Actor%20Object%20Reference))
  (bind _asbp_moving_object (Utilities|Casting|CastToBP_MovingObject (Variables|Default|GetTargetObject)))
  (Default|StartMoving _asbp_moving_object)
  (Class|BPIMyCharacter|MyCharacterOverlap(Message) OverlapActor (Utilities|GetDisplayName self)))

(event EventBeginPlay
  (EventDispatchers|BindEventtoOverlapBaseEventAction (delegate Custom|OverlapBaseEvent)))

(event EventDestroyObject
  (Actor|DestroyActor))

(fn ConstructionScript)