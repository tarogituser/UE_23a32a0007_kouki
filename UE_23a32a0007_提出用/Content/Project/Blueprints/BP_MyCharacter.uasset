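; Player character with Enhanced Input movement, look, jump and sprint, driving a HUD widget for HP, points and center messages.
; Damage reduces HP; death ragdolls the mesh, shows GameOver and reloads the level.
; Reaching the point goal starts all cached BP_MovingObject actors and hides the point display.
; A looping timer teleports the character to its spawn location when its mesh falls too low, with checkpoints updating that location.
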(event Custom|CheckDeadEvent
  (if (< (.z (Transformation|GetWorldLocation (Variables|Character|GetMesh))) -4e+02)
    (Transformation|SetActorLocation (Variables|Default|GetSpawnLocation) false false)))

(event Custom|Overlap%20Checkpoint
  (params (SpawnLocation :type Vector))
  (bind _playerui (Variables|Default|GetPlayerUI))
  (bind _centermessage (Variables|/Game/Project/Blueprints/UW_PlayerUI.UW_PlayerUI_C|GetCenterMessage _playerui))
  (Variables|Default|SetSpawnLocation SpawnLocation)
  (Widget|SetVisibility _centermessage "Visible")
  (Rendering|Components|TextRender|SetText _centermessage "Checkpoint Passed")
  (Utilities|FlowControl|Delay 4.0)
  (Widget|SetVisibility _centermessage "Hidden"))

(event Input|EnhancedActionEvents|EnhancedInputActionIA_MyLook
  (params (ActionValue :type Vector%202D%20Structure) (ElapsedSeconds :type Float%20%28double-precision%29) (TriggeredSeconds :type Float%20%28double-precision%29) (InputAction :type Input%20Action%20Object%20Reference :default "/Game/Project/Assets/Input/Actions/IA_MyLook.IA_MyLook"))
  (Pawn|Input|AddControllerYawInput (.x ActionValue))
  (Pawn|Input|AddControllerPitchInput (.y ActionValue)))

(event Input|EnhancedActionEvents|EnhancedInputActionIA_MyJump
  (params (ActionValue :type Boolean) (ElapsedSeconds :type Float%20%28double-precision%29) (TriggeredSeconds :type Float%20%28double-precision%29) (InputAction :type Input%20Action%20Object%20Reference :default "/Game/Project/Assets/Input/Actions/IA_MyJump.IA_MyJump"))
  (:Started
    (Character|Jump))
  (:Canceled
    (Character|StopJumping)))

(event Input|EnhancedActionEvents|EnhancedInputActionIA_MyMove
  (params (ActionValue :type Vector%202D%20Structure) (ElapsedSeconds :type Float%20%28double-precision%29) (TriggeredSeconds :type Float%20%28double-precision%29) (InputAction :type Input%20Action%20Object%20Reference :default "/Game/Project/Assets/Input/Actions/IA_MyMove.IA_MyMove"))
  (bind _returnvalue (Pawn|GetControlRotation :!class /Script/Engine.Pawn))
  (Pawn|Input|AddMovementInput (Math|Vector|GetRightVector (Math|Rotator|MakeRotator (.roll _returnvalue) 0.0 (.yaw _returnvalue))) (.x ActionValue) false)
  (Pawn|Input|AddMovementInput (Math|Vector|GetForwardVector (Math|Rotator|MakeRotator 0.0 0.0 (.yaw (Pawn|GetControlRotation :!class /Script/Engine.Pawn)))) (.y ActionValue) false))

(event Input|EnhancedActionEvents|EnhancedInputActionIA_MySprint
  (params (ActionValue :type Boolean) (ElapsedSeconds :type Float%20%28double-precision%29) (TriggeredSeconds :type Float%20%28double-precision%29) (InputAction :type Input%20Action%20Object%20Reference :default "/Game/Project/Assets/Input/Actions/IA_MySprint.IA_MySprint"))
  (bind _charactermovement (Variables|Character|GetCharacterMovement))
  (:Started
    (Variables|/Script/Engine.CharacterMovementComponent|SetMaxWalkSpeed _charactermovement 8e+02))
  (:Completed
    (Variables|/Script/Engine.CharacterMovementComponent|SetMaxWalkSpeed _charactermovement 6e+02)))

(event EventBeginPlay
  (bind _maxplayerhp (Variables|Default|GetMaxPlayerHp))
  (bind _returnvalue (UserInterface|CreateWidget "/Game/Project/Blueprints/UW_PlayerUI.UW_PlayerUI_C"))
  (bind _output_get (Variables|Default|SetPlayerUI _returnvalue))
  (UserInterface|Viewport|AddtoViewport _output_get 0)
  (Variables|Default|SetSpawnLocation (Transformation|GetActorLocation))
  (bind _output_get_2 (Variables|Default|SetPlayerHp _maxplayerhp))
  (Default|UpdateHPText (Variables|Default|GetPlayerUI) (Math|Float|Truncate _output_get_2) (Math|Float|Truncate _maxplayerhp))
  (Default|UpdatePointText (Variables|Default|GetPlayerUI) (Variables|Default|GetPlayerPoint) (Variables|Default|GetMaxPlayerPoint))
  (bind _outactors (Actor|GetAllActorsOfClass "/Game/Project/Blueprints/BP_MovingObject.BP_MovingObject_C"))
  (Variables|Default|SetMovingObjects _outactors)
  (Utilities|Time|SetTimerbyEvent (delegate Custom|CheckDeadEvent) 0.5 true))

(event Game|Damage|EventAnyDamage
  (params (Damage :type Float%20%28single-precision%29) (DamageType :type Damage%20Type%20Object%20Reference) (InstigatedBy :type Controller%20Object%20Reference) (DamageCauser :type Actor%20Object%20Reference))
  (bind _playerui (Variables|Default|GetPlayerUI))
  (bind _mesh (Variables|Character|GetMesh))
  (bind _maxplayerhp (Variables|Default|GetMaxPlayerHp))
  (bind _centermessage (Variables|/Game/Project/Blueprints/UW_PlayerUI.UW_PlayerUI_C|GetCenterMessage _playerui))
  (if (not (Variables|Default|Getb_Dead))
    (bind _output_get (Variables|Default|SetPlayerHp (Math|Float|Max(Float) 0.0 (- (Variables|Default|GetPlayerHp) Damage))))
    (Default|UpdateHPText (Variables|Default|GetPlayerUI) (Math|Float|Truncate _output_get) (Math|Float|Truncate _maxplayerhp))
    (Default|UpdateHpGauge (Variables|Default|GetPlayerUI) (/ _output_get _maxplayerhp))
    (if (<= (Variables|Default|GetPlayerHp) 0.0)
      (Variables|Default|Setb_Dead true)
      (Input|DisableInput 0)
      (Pawn|Components|CharacterMovement|DisableMovement (Variables|Character|GetCharacterMovement))
      (Collision|SetCollisionProfileName _mesh "Ragdoll" true :!class /Script/Engine.PrimitiveComponent)
      (Physics|SetSimulatePhysics _mesh true)
      (Rendering|Components|TextRender|SetText _centermessage "GameOver")
      (Widget|SetVisibility _centermessage "Visible")
      (Utilities|FlowControl|Delay 2.0)
      (Widget|SetVisibility _centermessage "Hidden")
      (Game|OpenLevel(byName) "MyGameLevel"))))

(event EventControllerChanged
  (params (OldController :type Controller%20Object%20Reference) (NewController :type Controller%20Object%20Reference))
  (bind _asplayer_controller (Utilities|Casting|CastToPlayerController NewController))
  (Input|AddMappingContext (PlayerController|LocalPlayerSubsystems|GetEnhancedInputLocalPlayerSubsystem _asplayer_controller) "/Game/Project/Assets/Input/IMC_MyInput.IMC_MyInput" 0 "(bIgnoreAllPressedKeysUntilRelease=True,bForceImmediately=False,bNotifyUserSettings=False)"))

(event EventMyCharacterOverlap
  (params (OverlapActorName :type String) (Point :type Integer))
  (bind _playerui (Variables|Default|GetPlayerUI))
  (bind _ismax (CallFunction|AddPlayerPoint Point))
  (if _ismax
    (for _array_element (Variables|Default|GetMovingObjects)
      (Default|StartMoving _array_element))
    (Widget|SetVisibility (Variables|/Game/Project/Blueprints/UW_PlayerUI.UW_PlayerUI_C|GetPointGauge _playerui) "Hidden")
    (Widget|SetVisibility (Variables|/Game/Project/Blueprints/UW_PlayerUI.UW_PlayerUI_C|GetPointText _playerui) "Hidden")))

(fn ConstructionScript)

(fn AddPlayerPoint
  (params (Point :type Integer))
  (bind _maxplayerpoint (Variables|Default|GetMaxPlayerPoint))
  (bind _output_get (Variables|Default|SetPlayerPoint (+ Point (Variables|Default|GetPlayerPoint))))
  (Default|UpdatePointText (Variables|Default|GetPlayerUI) _output_get _maxplayerpoint)
  (Default|UpdatePointGauge (Variables|Default|GetPlayerUI) (/ (Math|Conversions|ToFloat(Integer) _output_get) (Math|Conversions|ToFloat(Integer) _maxplayerpoint)))
  (return (>= (Variables|Default|GetPlayerPoint) (Variables|Default|GetMaxPlayerPoint))))