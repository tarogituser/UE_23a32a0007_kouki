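; BP_MovingObject is an actor whose Cube moves along a single axis when StartMoving is triggered.
; BReverse selects which timeline plays, Moving or ReverseMoving, and BHorizontal selects local X or Z as the axis.
; Each timeline update writes MovingValue into MoveVector and sets it as the Cube's relative location without sweeping, zeroing the other two axes.
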(event Custom|StartMoving
  (if (not (Variables|Default|Getb_Reverse))
    (bind _movingvalue (Timeline|Moving Play)
      (:Update
        (Utilities|FlowControl|Sequence
          (:then_0
            (if (Variables|Default|Getb_Horizontal)
              (Variables|Default|SetMoveVector (Math|Vector|MakeVector _movingvalue 0.0 0.0))
              (else
                (Variables|Default|SetMoveVector (Math|Vector|MakeVector 0.0 0.0 _movingvalue)))))
          (:then_1
            (Transformation|SetRelativeLocation (Variables|Default|GetCube) (Variables|Default|GetMoveVector) false false)))))
    (else
      (bind _movingvalue_2 (Timeline|Reverse%20Moving Play)
        (:Update
          (Utilities|FlowControl|Sequence
            (:then_0
              (if (Variables|Default|Getb_Horizontal)
                (Variables|Default|SetMoveVector (Math|Vector|MakeVector _movingvalue_2 0.0 0.0))
                (else
                  (Variables|Default|SetMoveVector (Math|Vector|MakeVector 0.0 0.0 _movingvalue_2)))))
            (:then_1
              (Transformation|SetRelativeLocation (Variables|Default|GetCube) (Variables|Default|GetMoveVector) false false))))))))

(fn ConstructionScript)