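; BP_Fire is a fire hazard actor that damages an actor once per second while it overlaps.
; On BeginPlay it runs the parent logic and binds handlers to the overlap begin and end base event actions.
; Overlap begin sets a single boolean and starts a Delay-based loop applying Damage to the overlapping actor, and overlap end clears the flag to stop it.
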(event Custom|Overlap%20Fire
  (params (OverlapActor :type Actor%20Object%20Reference))
  (bind _output_get (Variables|Default|Setb_Overlapping true))
  (if _output_get :!label _label
    (Game|Damage|ApplyDamage OverlapActor (Variables|Default|GetDamage) 0 0)
    (Utilities|FlowControl|Delay 1.0)
    (goto _label)))

(event Custom|Overlap%20End%20Fire
  (params (Overlap%20Actor :type Actor%20Object%20Reference))
  (Variables|Default|Setb_Overlapping false))

(event EventBeginPlay
  (|CallParentFunction)
  (EventDispatchers|BindEventtoOverlapBaseEventAction (delegate Custom|Overlap%20Fire))
  (EventDispatchers|BindEventtoOverlapEndBaseEventAction (delegate Custom|Overlap%20End%20Fire)))

(fn ConstructionScript
  (|CallParentFunction))