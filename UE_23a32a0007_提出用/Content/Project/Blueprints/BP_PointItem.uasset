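; Collectible point item that spins in place and awards points to the actor that overlaps it.
; Construction script reads the point value and mesh material from the DT_PointItem data table row named by PointItemDataName.
; A timeline drives the mesh's yaw.
; The parent's overlap dispatcher triggers pickup, which sends the item's name and points to the overlapping actor via MyCharacterOverlapMessage, plays a sound and destroys the item.
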(event Custom|OverlapPointItemEvent
  (params (OverlapActor :type Actor%20Object%20Reference))
  (Class|BPIMyCharacter|MyCharacterOverlap(Message) OverlapActor (Utilities|GetDisplayName self) (Variables|Default|GetPoint))
  (Audio|PlaySoundatLocation "/Game/Game_Item/Pick_Up/Wav/Wav_Ashorttactilesou1_wav.Wav_Ashorttactilesou1_wav" (Transformation|GetActorLocation) "0, 0, 0" 1.0 1.0 0.0 0 0 0 0)
  (Actor|DestroyActor))

(event EventBeginPlay
  (|CallParentFunction)
  (EventDispatchers|AssignOverlapBaseEventAction (delegate Custom|OverlapPointItemEvent))
  (bind _z (Timeline|Rotation PlayFromStart)
    (:Update
      (Transformation|SetRelativeRotation (Variables|Default|GetSTM_PointItem) (Math|Rotator|MakeRotator 0.0 0.0 _z) false false))))

(fn ConstructionScript
  (|CallParentFunction)
  (bind _returnvalue (Utilities|GetDataTableRow "/Game/Project/Blueprints/DT_PointItem.DT_PointItem" (Variables|Default|GetPointItemDataName))
    (:then
      (Variables|Default|SetPoint (.Point (Utilities|Struct|BreakST_PointItem _returnvalue)))
      (Rendering|Material|SetMaterial (Variables|Default|GetSTM_PointItem) 0 (.Material (Utilities|Struct|BreakST_PointItem _returnvalue))))))